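; BP_DialogueMapPawn is the player pawn for an Inworld dialogue map, connecting the player to the map's AI character.
; On BeginPlay it finds the session controller and waits for session creation and loading, binding delegates and also calling each handler immediately to cover already-ready states.
; Once loaded, the server sets the map character as the player component's target, and the locally controlled pawn creates the dialogue widget.
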(event Custom|OnLoaded
  (params (bLoaded :type Boolean))
  (if bLoaded
    (EventDispatchers|UnbindEventfromOnSessionLoadedDelegate (Variables|Default|GetInworldSessionComponent) (delegate Custom|OnLoaded))
    (Utilities|FlowControl|Sequence
      (:then_0
        (if (Networking|IsServer)
          (bind _returnvalue (Actor|GetActorOfClass "/InworldAI/Dialogue/BP_DialogueMapCharacter.BP_DialogueMapCharacter_C"))
          (Class|InworldPlayerComponent|SetTargetInworldCharacter (Variables|Default|GetInworldPlayerComponent) (Variables|/InworldAI/Dialogue/BP_DialogueMapCharacter.BP_DialogueMapCharacter_C|GetInworldCharacterComponent _returnvalue))))
      (:then_1
        (if (Pawn|IsLocallyControlled)
          (bind _returnvalue_2 (Actor|GetActorOfClass "/InworldAI/Dialogue/BP_DialogueMapCharacter.BP_DialogueMapCharacter_C"))
          (bind _returnvalue_3 (UserInterface|CreateWidget "/InworldAI/Dialogue/WBP_DialogueWidget.WBP_DialogueWidget_C" (Game|GetPlayerController 0) _returnvalue_2 self))
          (UserInterface|Viewport|AddtoViewport _returnvalue_3 0))))))

(event Custom|AwaitLoaded
  (bind _inworldsessioncomponent (Variables|Default|GetInworldSessionComponent))
  (EventDispatchers|BindEventtoOnSessionLoadedDelegate _inworldsessioncomponent (EventDispatchers|CreateEvent :!event Custom|OnLoaded))
  (CallFunction|OnLoaded (Class|InworldSessionComponent|GetIsLoaded _inworldsessioncomponent)))

(event Custom|OnSessionCreated
  (bind _inworldsessioncomponent (Variables|Default|GetInworldSessionComponent))
  (Utilities|IsValid _inworldsessioncomponent
    (:Is%20Valid
      (EventDispatchers|UnbindEventfromOnSessionCreatedDelegate _inworldsessioncomponent (delegate Custom|OnSessionCreated))
      (CallFunction|AwaitLoaded))))

(event EventBeginPlay
  (|CallParentFunction)
  (bind _returnvalue (Actor|GetActorOfClass "/InworldAI/Dialogue/BP_DialogueInworldSessionController.BP_DialogueInworldSessionController_C"))
  (bind _output_get (Variables|Default|SetInworldSessionComponent (Variables|/InworldAI/Dialogue/BP_DialogueInworldSessionController.BP_DialogueInworldSessionController_C|GetInworldSession _returnvalue)))
  (EventDispatchers|BindEventtoOnSessionCreatedDelegate _output_get (EventDispatchers|CreateEvent :!event Custom|OnSessionCreated))
  (CallFunction|OnSessionCreated))

(fn ConstructionScript)
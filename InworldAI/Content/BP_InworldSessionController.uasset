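; Actor that controls an Inworld AI session, starting it for a configured scene when play begins.
; On BeginPlay the server sets the session's auth from an API key and secret, fills the player profile with the player name, then starts the session.
; Connection state changes are printed for debugging, and GetInworldSession exposes the session to other code.
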(event OnSessionConnectionStateChangedDelegate(InworldSession)
  (params (ConnectionState :type EInworldConnectionState%20Enum :default "Idle"))
  (Development|PrintString (Utilities|String|Append "Connection state: " (Utilities|String|EnumtoString ConnectionState))))

(event EventBeginPlay
  (bind _apikey (Variables|Default|GetApiKey))
  (|CallParentFunction)
  (if (Networking|IsServer)
    (Variables|/Script/InworldAIIntegration.InworldSessionComponent|SetAuth (Variables|Default|GetInworldSession) (Utilities|Struct|MakeInworldAuth "" (.apikey _apikey) (.apisecret _apikey)))
    (Variables|/Script/InworldAIIntegration.InworldSessionComponent|SetPlayerProfile (Variables|Default|GetInworldSession) (Utilities|Struct|MakeInworldPlayerProfile (Variables|Default|GetPlayer%20Name) "" "" 0))
    (Class|InworldSessionComponent|StartSession (Variables|Default|GetInworldSession) (Variables|Default|GetSceneName))))

(fn ConstructionScript)

(fn GetInworldSession
  (return (Class|InworldBlueprintFunctionLibrary|ToSession(InworldSessionComponent) (Variables|Default|GetInworldSession))))
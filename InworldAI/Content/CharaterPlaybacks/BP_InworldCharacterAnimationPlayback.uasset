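; Inworld character playback that plays gesture montages on the owning Character's mesh while it speaks.
; When an utterance starts and no gesture is playing, it selects a montage from data tables, preferring custom gestures over emotion-based ones.
; When a montage ends, it starts another emotion gesture if enough utterance audio remains.
; Interruptions stop the montage instantly, and emotion changes clear the cached emotion montages.
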(event EventBeginPlay
  (|CallParentFunction)
  (bind _ascharacter (Utilities|Casting|CastToCharacter (Class|InworldCharacterPlayback|GetOwner)))
  (bind _output_get (Variables|Default|SetOwner%20As%20Character _ascharacter))
  (Variables|Default|SetMesh (Variables|/Script/Engine.Character|GetMesh _output_get))
  (Utilities|IsValid (Class|InworldCharacterPlayback|GetCharacterComponent)
    (:Is%20Valid
      (EventDispatchers|BindEventtoOnEmotionalBehaviorChanged (Class|InworldCharacterPlayback|GetCharacterComponent) (EventDispatchers|CreateEvent :!event EmotionChanged))
      (bind _output_get_2 (Variables|Components|SetAudioPlayback (Class|InworldCharacterComponent|GetPlayback (Class|InworldCharacterPlayback|GetCharacterComponent) "/Script/InworldAIIntegration.InworldCharacterPlaybackAudio")))
      (Utilities|IsValid _output_get_2
        (:Is%20Valid
          (EventDispatchers|BindEventtoOnUtteranceStarted _output_get_2 (EventDispatchers|CreateEvent :!event UtteranceStarted))
          (EventDispatchers|BindEventtoOnUtteranceInterrupted _output_get_2 (EventDispatchers|CreateEvent :!event UtteranceInterrupted)))))))

(fn EmotionChanged
  (params (EmotionalBehavior :type EInworldCharacterEmotionalBehavior%20Enum :default "NEUTRAL") (Strength :type EInworldCharacterEmotionStrength%20Enum :default "UNSPECIFIED"))
  (Utilities|Array|Clear (Variables|Default|GetCurrentEmotionMontages)))

(fn UtteranceStarted
  (params (Duration :type Float%20%28single-precision%29) (CustomGesture :type String))
  (bind _returnvalue (Class|InworldCharacterPlayback|GetCharacterComponent))
  (bind _mesh (Variables|Default|GetMesh))
  (Utilities|IsValid (Variables|Gesture|GetCurrentGestureMontage) ; Ensure montage is not interrupted by new gesture
    (:Is%20Not%20Valid
      (LocalVariables|SetGestureMontage (Class|InworldCharacterAnimationsLib|GetMontageforCustomGesture (Variables|DataTable|GetGesture%20Animation%20DT) CustomGesture Duration true true))
      (LocalVariables|SetEmotionMontage (Class|InworldCharacterAnimationsLib|GetMontageforEmotion (Variables|DataTable|GetEmotion%20Animation%20DT) (Class|InworldCharacterComponent|GetEmotionalBehavior _returnvalue) (Class|InworldCharacterComponent|GetEmotionStrength _returnvalue) Duration true true (Variables|Default|GetCurrentEmotionMontages)))
      (Utilities|IsValid (select (or (not (Utilities|IsValid (LocalVariables|GetGestureMontage))) (Utilities|Array|IsEmpty CustomGesture)) (LocalVariables|GetEmotionMontage) (LocalVariables|GetGestureMontage))
        (:Is%20Valid
          (Utilities|IsValid _mesh
            (:Is%20Valid
              (Variables|Gesture|SetCurrentGestureMontage (select (or (not (Utilities|IsValid (LocalVariables|GetGestureMontage))) (Utilities|Array|IsEmpty CustomGesture)) (LocalVariables|GetEmotionMontage) (LocalVariables|GetGestureMontage))) ; Find and set the best montage for the gesture
              (EventDispatchers|BindEventtoOnMontageEnded (Components|SkeletalMesh|GetAnimInstance _mesh) (EventDispatchers|CreateEvent :!event OnMontageEnd)) ; Listen for the montage to end
              (Class|AnimInstance|MontagePlaywithBlendin (Components|SkeletalMesh|GetAnimInstance (Variables|Default|GetMesh)) (Variables|Gesture|GetCurrentGestureMontage) (Variables|Gesture|GetMontageBlendInSettings) 1.0 "MontageLength" 0.0 true))))))))

(fn UtteranceInterrupted
  (Utilities|IsValid (Variables|Gesture|GetCurrentGestureMontage)
    (:Is%20Valid
      (Animation|Montage|MontageStop (Components|SkeletalMesh|GetAnimInstance (Variables|Default|GetMesh)) 0.0 (Variables|Gesture|GetCurrentGestureMontage))
      (Variables|Gesture|SetCurrentGestureMontage 0))))

(fn OnMontageEnd
  (params (Montage :type Anim%20Montage%20Object%20Reference) (bInterrupted :type Boolean))
  (if (== Montage (Variables|Gesture|GetCurrentGestureMontage))
    (Variables|Gesture|SetCurrentGestureMontage 0)
    (EventDispatchers|UnbindEventfromOnMontageEnded (Components|SkeletalMesh|GetAnimInstance (Variables|Default|GetMesh)) (EventDispatchers|CreateEvent :!event OnMontageEnd))
    (CallFunction|OnGestureFinished)))

(fn OnGestureFinished
  (CallFunction|TrytoContinueGesturing))

(fn TrytoContinueGesturing
  (bind _returnvalue (Class|InworldCharacterPlayback|GetCharacterComponent))
  (bind _returnvalue_2 (Class|InworldCharacterComponent|GetPlayback _returnvalue "/Script/InworldAIIntegration.InworldCharacterPlaybackAudio"))
  (bind _returnvalue_3 (Class|InworldCharacterPlaybackAudio|GetRemainingTimeforCurrentUtterance _returnvalue_2))
  (if (< (Variables|Gesture|GetRemainingTimeToContinueGesture) _returnvalue_3)
    (CallFunction|UtteranceStarted _returnvalue_3)))
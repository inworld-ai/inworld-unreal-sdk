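; A widget component that shows chat bubbles for an Inworld AI character's conversation.
; On BeginPlay it caches its WBP_ChatBubbles widget and, if the owner has an InworldCharacterComponent, binds to that component's utterance, utterance interrupt and player talk events.
; Each handler forwards its event data straight to the widget, so the component serves only as a bridge between character and UI.
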(event Custom|OnCharacterUtterance
  (params (Utterance :type Character%20Message%20Utterance%20Structure%20%28by%20ref%29))
  (Default|OnCharacterUtterance (Variables|Default|GetChatBubblesWidget) Utterance))

(event Custom|OnCharacterUtteranceInterrupt
  (params (Utterance :type Character%20Message%20Utterance%20Structure%20%28by%20ref%29))
  (Default|OnCharacterUtteranceInterrupt (Variables|Default|GetChatBubblesWidget) Utterance))

(event Custom|OnCharacterPlayerTalk
  (params (PlayerTalk :type Character%20Message%20Player%20Talk%20Structure%20%28by%20ref%29))
  (Default|OnPlayerTalk (Variables|Default|GetChatBubblesWidget) PlayerTalk))

(event EventBeginPlay
  (bind _returnvalue (Components|GetOwner))
  (bind _returnvalue_2 (UserInterface|GetUserWidgetObject))
  (bind _returnvalue_3 (Actor|GetComponentbyClass _returnvalue "/Script/InworldAIIntegration.InworldCharacterComponent"))
  (|CallParentFunction)
  (Utilities|IsValid _returnvalue_2
    (:Is%20Valid
      (bind _aswbp_chat_bubbles (Utilities|Casting|CastToWBP_ChatBubbles _returnvalue_2))
      (Variables|Default|SetChatBubblesWidget _aswbp_chat_bubbles)
      (Utilities|IsValid _returnvalue_3
        (:Is%20Valid
          (EventDispatchers|AssignOnUtterance _returnvalue_3 (EventDispatchers|CreateEvent :!event Custom|OnCharacterUtterance))
          (EventDispatchers|AssignOnUtteranceInterrupt _returnvalue_3 (EventDispatchers|CreateEvent :!event Custom|OnCharacterUtteranceInterrupt))
          (EventDispatchers|AssignOnPlayerTalk _returnvalue_3 (EventDispatchers|CreateEvent :!event Custom|OnCharacterPlayerTalk)))))))
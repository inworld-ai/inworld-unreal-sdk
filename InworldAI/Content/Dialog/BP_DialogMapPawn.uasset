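; BP_DialogMapPawn is the player pawn for a dialog map where the player talks to an Inworld AI character.
; On BeginPlay it finds the session controller's Inworld session and waits through delegates for it to be created, then loaded.
; Once loaded, the server sets the player component's target to the map's dialog character.
; The locally controlled pawn creates the dialog widget and switches to UI-only input focused on its text box.
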(event Custom|OnLoaded
  (params (bLoaded :type Boolean))
  (if bLoaded
    (EventDispatchers|UnbindEventfromOnSessionLoadedDelegate (Variables|Default|GetInworldSessionComponent) (delegate Custom|OnLoaded))
    (Utilities|FlowControl|Sequence
      (:then_0
        (if (Networking|IsServer)
          (bind _returnvalue (Actor|GetActorOfClass "/InworldAI/Dialog/BP_DialogMapCharacter.BP_DialogMapCharacter_C"))
          (Class|InworldPlayerComponent|SetTargetInworldCharacter (Variables|Default|GetInworldPlayerComponent) (Variables|/InworldAI/Dialog/BP_DialogMapCharacter.BP_DialogMapCharacter_C|GetInworldCharacterComponent _returnvalue))))
      (:then_1
        (if (Pawn|IsLocallyControlled)
          (bind _returnvalue_2 (Actor|GetActorOfClass "/InworldAI/Dialog/BP_DialogMapCharacter.BP_DialogMapCharacter_C"))
          (bind _returnvalue_3 (UserInterface|CreateWidget "/InworldAI/Dialog/WBP_DialogWidget.WBP_DialogWidget_C" (Game|GetPlayerController 0) _returnvalue_2 self))
          (UserInterface|Viewport|AddtoViewport _returnvalue_3 0)
          (Input|SetInputModeUIOnly (Game|GetPlayerController 0) (Variables|/InworldAI/Dialog/WBP_DialogWidget.WBP_DialogWidget_C|GetInputText _returnvalue_3) "DoNotLock"))))))

(event Custom|AwaitLoaded
  (bind _inworldsessioncomponent (Variables|Default|GetInworldSessionComponent))
  (EventDispatchers|BindEventtoOnSessionLoadedDelegate _inworldsessioncomponent (EventDispatchers|CreateEvent :!event Custom|OnLoaded))
  (CallFunction|OnLoaded (Class|InworldSessionComponent|GetIsLoaded _inworldsessioncomponent)))

(event Custom|OnSessionCreated
  (bind _inworldsessioncomponent (Variables|Default|GetInworldSessionComponent))
  (Utilities|IsValid _inworldsessioncomponent
    (:Is%20Valid
      (EventDispatchers|UnbindEventfromOnSessionCreatedDelegate _inworldsessioncomponent (delegate Custom|OnSessionCreated))
      (CallFunction|AwaitLoaded))))

(event EventBeginPlay
  (|CallParentFunction)
  (bind _returnvalue (Actor|GetActorOfClass "/InworldAI/Dialog/BP_DialogInworldSessionController.BP_DialogInworldSessionController_C"))
  (bind _output_get (Variables|Default|SetInworldSessionComponent (Variables|/InworldAI/Dialog/BP_DialogInworldSessionController.BP_DialogInworldSessionController_C|GetInworldSession _returnvalue)))
  (EventDispatchers|BindEventtoOnSessionCreatedDelegate _output_get (EventDispatchers|CreateEvent :!event Custom|OnSessionCreated))
  (CallFunction|OnSessionCreated))

(fn ConstructionScript)
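; Component that animates an Innequin character's texture-based face from its owner's Inworld emotion and lip-sync data.
; Emotional behaviors collapse into fewer emotions, which pick data-table textures for brow, eye, nose and mouth dynamic materials and play an emote flipbook.
; The strongest viseme overrides the mouth, using half-shape textures at low weight with full-shape fallback.
; A randomized timer calls SetBlinking, whose body is empty here.
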(event EventBeginPlay
  (|CallParentFunction)
  (Components|InitComponents)
  (Material|CreateDynamicMaterialInstances)
  (Emotion|BindEmotionEvent)
  (Viseme|BindVisemeEvent)
  (Utilities|FlowControl|Delay 3.0)
  (Blink|Blink))

(fn CreateDynamicMaterialInstances
  (bind _material_instance (Utilities|CreateDynamicMaterialInstance (Variables|Default|GetMesh) (Rendering|Material|GetMaterialIndex (Variables|Default|GetMesh) "mtl_faceshapes_mouth"))
    (:%20%20
      (Variables|Material|SetMouth%20Material%20Instance _material_instance)
      (bind _material_instance_2 (Utilities|CreateDynamicMaterialInstance (Variables|Default|GetMesh) (Rendering|Material|GetMaterialIndex (Variables|Default|GetMesh) "mtl_faceshapes_eyes"))
        (:%20%20
          (Variables|Material|SetEyes%20Material%20Instance _material_instance_2)
          (bind _material_instance_3 (Utilities|CreateDynamicMaterialInstance (Variables|Default|GetMesh) (Rendering|Material|GetMaterialIndex (Variables|Default|GetMesh) "mtl_faceshapes_brows"))
            (:%20%20
              (Variables|Material|SetBrows%20Material%20Instance _material_instance_3)
              (bind _material_instance_4 (Utilities|CreateDynamicMaterialInstance (Variables|Default|GetMesh) (Rendering|Material|GetMaterialIndex (Variables|Default|GetMesh) "mtl_faceshapes_nose"))
                (:%20%20
                  (Variables|Material|SetNose%20Material%20Instance _material_instance_4))))))))))

(fn BindEmotionEvent
  (bind _inworldcharactercomponent (Variables|Default|GetInworldCharacterComponent))
  (EventDispatchers|BindEventtoOnEmotionalBehaviorChanged _inworldcharactercomponent (EventDispatchers|CreateEvent :!event OnEmotionalBehaviorChanged))
  (Emotion|OnEmotionalBehaviorChanged (Class|InworldCharacterComponent|GetEmotionalBehavior _inworldcharactercomponent) (Class|InworldCharacterComponent|GetEmotionStrength _inworldcharactercomponent)))

(fn Blink
  (Utilities|Time|SetTimerbyEvent (EventDispatchers|CreateEvent :!event Blink) (select (Variables|Blink|GetBlinking) (Math|Random|RandomFloatinRange 3.0 5.0) (Math|Random|RandomFloatinRange 0.1 0.25)))
  (Blink|SetBlinking (not (Variables|Blink|GetBlinking))))

(fn BindVisemeEvent
  (bind _returnvalue (Components|GetOwner))
  (bind _inworldcharactercomponent (Variables|Default|GetInworldCharacterComponent))
  (bind _returnvalue_2 (Class|InworldCharacterComponent|GetPlayback _inworldcharactercomponent "/Script/InworldAIIntegration.InworldCharacterPlaybackAudio"))
  (bind _returnvalue_3 (Actor|GetComponentbyClass _returnvalue "/Script/InworldAIIntegration.InworldCharacterAudioComponent"))
  (Utilities|IsValid _returnvalue_3
    (:Is%20Valid
      (EventDispatchers|BindEventtoOnVisemeBlendsUpdated _returnvalue_3 (EventDispatchers|CreateEvent :!event OnVisemeBlendsUpdated)))
    (:Is%20Not%20Valid
      (EventDispatchers|BindEventtoOnVisemeBlendsUpdated _returnvalue_2 (EventDispatchers|CreateEvent :!event OnVisemeBlendsUpdated))
      (Viseme|OnVisemeBlendsUpdated (Class|InworldCharacterPlaybackAudio|GetVismeBlends _returnvalue_2)))))

(fn SetBlinking
  (params (Blinking :type Boolean)))

(fn SetMaterialTextures
  (bind _blinking (Variables|Blink|GetBlinking))
  (bind _viseme (Variables|Viseme|GetViseme))
  (bind _viseme_2 (Variables|Viseme|GetViseme))
  (Utilities|FlowControl|Sequence
    (:then_0
      (bind _returnvalue (Utilities|GetDataTableRow "/InworldInnequin/Face/DT_InnequinEmotion_Brow.DT_InnequinEmotion_Brow" (Variables|Emotion|GetEmotion))
        (:then
          (Utilities|SetMaterialTextureParamaters (Variables|Material|GetBrows%20Material%20Instance) (.albedotexture (.brow _returnvalue)) (.opacitymasktexture (.brow _returnvalue))))))
    (:then_1
      (bind _returnvalue_2 (Utilities|GetDataTableRow "/InworldInnequin/Face/DT_InnequinEmotion_Eyes.DT_InnequinEmotion_Eyes" (Variables|Emotion|GetEmotion))
        (:then
          (Utilities|SetMaterialTextureParamaters (Variables|Material|GetEyes%20Material%20Instance) (select _blinking (.albedotexture (.closed _returnvalue_2)) (.albedotexture (.open _returnvalue_2))) (select _blinking (.opacitymasktexture (.closed _returnvalue_2)) (.opacitymasktexture (.open _returnvalue_2)))))))
    (:then_2
      (bind _returnvalue_3 (Utilities|GetDataTableRow "/InworldInnequin/Face/DT_InnequinEmotion_Nose.DT_InnequinEmotion_Nose" (Variables|Emotion|GetEmotion))
        (:then
          (Utilities|SetMaterialTextureParamaters (Variables|Material|GetNose%20Material%20Instance) (.albedotexture (.nose _returnvalue_3)) (.opacitymasktexture (.nose _returnvalue_3))))))
    (:then_3
      (if (Utilities|Enum|Equal(Enum) (Variables|Viseme|GetViseme) "NewEnumerator15")
        (bind _returnvalue_4 (Utilities|GetDataTableRow "/InworldInnequin/Face/DT_InnequinEmotion_Mouth.DT_InnequinEmotion_Mouth" (Variables|Emotion|GetEmotion))
          (:then
            (Utilities|SetMaterialTextureParamaters (Variables|Material|GetMouth%20Material%20Instance) (.albedotexture (.mouth _returnvalue_4)) (.opacitymasktexture (.mouth _returnvalue_4)))))
        (elif (Variables|Viseme|GetIsHalfViseme)
          (bind _returnvalue_5 (Utilities|GetDataTableRow "/InworldInnequin/Face/DT_InnequinEmotion_VisemeHalf.DT_InnequinEmotion_VisemeHalf" (Variables|Emotion|GetEmotion))
            (:then
              (Utilities|SetMaterialTextureParamaters (Variables|Material|GetMouth%20Material%20Instance) (Utilities|Select :Index _viseme_2 :NewEnumerator9 (.albedotexture (.pp _returnvalue_5)) :NewEnumerator4 (.albedotexture (.ff _returnvalue_5)) :NewEnumerator13 (.albedotexture (.th _returnvalue_5)) :NewEnumerator2 (.albedotexture (.dd _returnvalue_5)) :NewEnumerator6 (.albedotexture (.kk _returnvalue_5)) :NewEnumerator1 (.albedotexture (.ch _returnvalue_5)) :NewEnumerator12 (.albedotexture (.ss _returnvalue_5)) :NewEnumerator7 (.albedotexture (.nn _returnvalue_5)) :NewEnumerator10 (.albedotexture (.rr _returnvalue_5)) :NewEnumerator0 (.albedotexture (.aa _returnvalue_5)) :NewEnumerator3 (.albedotexture (.e _returnvalue_5)) :NewEnumerator5 (.albedotexture (.i _returnvalue_5)) :NewEnumerator8 (.albedotexture (.o _returnvalue_5)) :NewEnumerator14 (.albedotexture (.u _returnvalue_5)) :NewEnumerator15 0) (Utilities|Select :Index _viseme_2 :NewEnumerator9 (.opacitymasktexture (.pp _returnvalue_5)) :NewEnumerator4 (.opacitymasktexture (.ff _returnvalue_5)) :NewEnumerator13 (.opacitymasktexture (.th _returnvalue_5)) :NewEnumerator2 (.opacitymasktexture (.dd _returnvalue_5)) :NewEnumerator6 (.opacitymasktexture (.kk _returnvalue_5)) :NewEnumerator1 (.opacitymasktexture (.ch _returnvalue_5)) :NewEnumerator12 (.opacitymasktexture (.ss _returnvalue_5)) :NewEnumerator7 (.opacitymasktexture (.nn _returnvalue_5)) :NewEnumerator10 (.opacitymasktexture (.rr _returnvalue_5)) :NewEnumerator0 (.opacitymasktexture (.aa _returnvalue_5)) :NewEnumerator3 (.opacitymasktexture (.e _returnvalue_5)) :NewEnumerator5 (.opacitymasktexture (.i _returnvalue_5)) :NewEnumerator8 (.opacitymasktexture (.o _returnvalue_5)) :NewEnumerator14 (.opacitymasktexture (.u _returnvalue_5)) :NewEnumerator15 0)))
            (:RowNotFound
              (bind _returnvalue_6 (Utilities|GetDataTableRow "/InworldInnequin/Face/DT_InnequinEmotion_Viseme.DT_InnequinEmotion_Viseme" (Variables|Emotion|GetEmotion) :!label _label)
                (:then
                  (Utilities|SetMaterialTextureParamaters (Variables|Material|GetMouth%20Material%20Instance) (Utilities|Select :Index _viseme :NewEnumerator9 (.albedotexture (.pp _returnvalue_6)) :NewEnumerator4 (.albedotexture (.ff _returnvalue_6)) :NewEnumerator13 (.albedotexture (.th _returnvalue_6)) :NewEnumerator2 (.albedotexture (.dd _returnvalue_6)) :NewEnumerator6 (.albedotexture (.kk _returnvalue_6)) :NewEnumerator1 (.albedotexture (.ch _returnvalue_6)) :NewEnumerator12 (.albedotexture (.ss _returnvalue_6)) :NewEnumerator7 (.albedotexture (.nn _returnvalue_6)) :NewEnumerator10 (.albedotexture (.rr _returnvalue_6)) :NewEnumerator0 (.albedotexture (.aa _returnvalue_6)) :NewEnumerator3 (.albedotexture (.e _returnvalue_6)) :NewEnumerator5 (.albedotexture (.i _returnvalue_6)) :NewEnumerator8 (.albedotexture (.o _returnvalue_6)) :NewEnumerator14 (.albedotexture (.u _returnvalue_6)) :NewEnumerator15 0) (Utilities|Select :Index _viseme :NewEnumerator9 (.opacitymasktexture (.pp _returnvalue_6)) :NewEnumerator4 (.opacitymasktexture (.ff _returnvalue_6)) :NewEnumerator13 (.opacitymasktexture (.th _returnvalue_6)) :NewEnumerator2 (.opacitymasktexture (.dd _returnvalue_6)) :NewEnumerator6 (.opacitymasktexture (.kk _returnvalue_6)) :NewEnumerator1 (.opacitymasktexture (.ch _returnvalue_6)) :NewEnumerator12 (.opacitymasktexture (.ss _returnvalue_6)) :NewEnumerator7 (.opacitymasktexture (.nn _returnvalue_6)) :NewEnumerator10 (.opacitymasktexture (.rr _returnvalue_6)) :NewEnumerator0 (.opacitymasktexture (.aa _returnvalue_6)) :NewEnumerator3 (.opacitymasktexture (.e _returnvalue_6)) :NewEnumerator5 (.opacitymasktexture (.i _returnvalue_6)) :NewEnumerator8 (.opacitymasktexture (.o _returnvalue_6)) :NewEnumerator14 (.opacitymasktexture (.u _returnvalue_6)) :NewEnumerator15 0))))))
          (else
            (goto _label)))))))

(fn OnEmotionalBehaviorChanged
  (params (EmotionalBehavior :type EInworldCharacterEmotionalBehavior%20Enum :default "NEUTRAL") (Strength :type EInworldCharacterEmotionStrength%20Enum :default "UNSPECIFIED"))
  (switch Utilities|FlowControl|Switch|SwitchonEInworldCharacterEmotionalBehavior EmotionalBehavior
    (:NEUTRAL
      (Emotion|SetEmotion "Neutral" :!label _label))
    (:DISGUST
      (Emotion|SetEmotion "Angry" :!label _label_2))
    (:CONTEMPT
      (goto _label_2))
    (:BELLIGERENCE
      (goto _label_2))
    (:DOMINEERING
      (goto _label_2))
    (:CRITICISM
      (goto _label_2))
    (:ANGER
      (goto _label_2))
    (:TENSION
      (Emotion|SetEmotion "Fear"))
    (:TENSE_HUMOR
      (Emotion|SetEmotion "Humor" :!label _label_3))
    (:DEFENSIVENESS
      (goto _label))
    (:WHINING
      (Emotion|SetEmotion "Sad" :!label _label_4))
    (:SADNESS
      (goto _label_4))
    (:STONEWALLING
      (goto _label_2))
    (:INTEREST
      (Emotion|SetEmotion "Joy" :!label _label_5))
    (:VALIDATION
      (Emotion|SetEmotion "Affection" :!label _label_6))
    (:AFFECTION
      (goto _label_6))
    (:HUMOR
      (goto _label_3))
    (:SURPRISE
      (goto _label))
    (:JOY
      (goto _label_5))))

(fn SetEmotion
  (params (Emotion :type Name))
  (Variables|Emotion|SetEmotion Emotion)
  (Material|SetMaterialTextures)
  (Emotion|PlayEmoteFlipbook))

(fn PlayEmoteFlipbook
  (bind _returnvalue (Utilities|GetDataTableRow "/InworldInnequin/Emote/DT_InnequinEmoteData.DT_InnequinEmoteData" (Variables|Emotion|GetEmotion))
    (:then
      (Sprite|SetFlipbook (Variables|Default|GetPaperFlipbookEmote) (.emote _returnvalue))
      (Transformation|SetRelativeLocation (Variables|Default|GetPaperFlipbookEmote) (.emoterelativelocation _returnvalue) false true)
      (Components|Timeline|SetLooping (Variables|Default|GetPaperFlipbookEmote) false)
      (Components|Timeline|PlayfromStart (Variables|Default|GetPaperFlipbookEmote)))))

(fn OnVisemeBlendsUpdated
  (params (VisemeBlends :type Inworld%20Character%20Viseme%20Blends%20Structure))
  (bind _array (Utilities|Array|MakeArray (.pp VisemeBlends) (.ff VisemeBlends) (.th VisemeBlends) (.dd VisemeBlends) (.kk VisemeBlends) (.ch VisemeBlends) (.ss VisemeBlends) (.nn VisemeBlends) (.rr VisemeBlends) (.aa VisemeBlends) (.e VisemeBlends) (.i VisemeBlends) (.o VisemeBlends) (.u VisemeBlends) (.stop VisemeBlends)))
  (bind (_indexofmaxvalue _maxvalue) (Math|Float|MaxOfFloatArray _array))
  (Viseme|SetViseme (|IndexToVisemeCode _indexofmaxvalue) (<= _maxvalue (LocalVariables|GetHalfVisemeValue))))

(fn SetViseme
  (params (Viseme :type E_InnequinVisemes%20Enum :default "NewEnumerator9") (Half :type Boolean))
  (Variables|Viseme|SetViseme Viseme)
  (Variables|Viseme|SetIsHalfViseme Half)
  (Material|SetMaterialTextures))

(fn InitComponents
  (Variables|Default|SetInworldCharacterComponent (Actor|GetComponentbyClass (Components|GetOwner) "/Script/InworldAIIntegration.InworldCharacterComponent"))
  (Variables|Default|SetPaperFlipbookEmote (Actor|GetComponentbyClass (Components|GetOwner) "/Script/Paper2D.PaperFlipbookComponent"))
  (Variables|Default|SetMesh (Actor|GetComponentbyClass (Components|GetOwner) "/Script/Engine.SkeletalMeshComponent")))